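; Level transition actor that moves Marisa to another map, triggered by an action event or, when Auto is set, by overlapping its box.
; It saves the player's status to the game instance along with the exit info and next and current level names.
; It then shows a fade widget, starts streaming the Loading level and opens it after a short delay.
; Only the action path checks that NextLevel is set.
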(event OnComponentBeginOverlap(Box)
  (params (OtherActor :type Actor%20Object%20Reference) (OtherComp :type Primitive%20Component%20Object%20Reference) (OtherBodyIndex :type Integer) (bFromSweep :type Boolean) (SweepResult :type Hit%20Result%20Structure%20%28by%20ref%29))
  (bind _returnvalue (Game|GetGameInstance))
  (bind _asgmae_instance_bp (Utilities|Casting|CastToGmaeInstance_BP _returnvalue))
  (bind _asmarisa_bp (Utilities|Casting|CastToMarisa_BP OtherActor))
  (if (Variables|Default|Getauto)
    (Utilities|SavePlayerStautos _asmarisa_bp)
    (Utilities|FlowControl|Delay 0.1)
    (CallFunction|RemoveWidget)
    (Variables|/Game/BluePrints/GmaeInstance_BP.GmaeInstance_BP_C|SetmapMoveOut _asgmae_instance_bp (Variables|Default|GetmapMoveOut))
    (Variables|/Game/BluePrints/GmaeInstance_BP.GmaeInstance_BP_C|SetnextLevelName _asgmae_instance_bp (Variables|Default|GetnextLevel))
    (bind _returnvalue_2 (Game|GetCurrentLevelName true))
    (Variables|/Game/BluePrints/GmaeInstance_BP.GmaeInstance_BP_C|SetbeforeLevelName _asgmae_instance_bp (Utilities|String|StringToName _returnvalue_2))
    (bind _returnvalue_3 (UserInterface|CreateWidget "/Game/BluePrints/UMG/FadeWidget_BP.FadeWidget_BP_C" 0 false))
    (UserInterface|Viewport|AddtoViewport _returnvalue_3 0)
    (Utilities|FlowControl|Sequence
      (:then_0
        (Game|LoadStreamLevel(byName) "Loading" true))
      (:then_1
        (Utilities|FlowControl|Delay 0.5)
        (Game|OpenLevel(byName) "Loading")))))

(event EventBeginPlay
  (Variables|Default|SethideEventIcon true))

(event EventActionEvent
  (params (marisa :type Marisa%20BP%20Object%20Reference))
  (bind _returnvalue (Game|GetGameInstance))
  (bind _asgmae_instance_bp (Utilities|Casting|CastToGmaeInstance_BP _returnvalue))
  (if (not (Utilities|Name|Equal(Name) (Variables|Default|GetnextLevel) "None"))
    (Utilities|SavePlayerStautos marisa)
    (Utilities|FlowControl|Delay 0.1)
    (CallFunction|RemoveWidget)
    (Variables|/Game/BluePrints/GmaeInstance_BP.GmaeInstance_BP_C|SetmapMoveOut _asgmae_instance_bp (Variables|Default|GetmapMoveOut))
    (Variables|/Game/BluePrints/GmaeInstance_BP.GmaeInstance_BP_C|SetnextLevelName _asgmae_instance_bp (Variables|Default|GetnextLevel))
    (bind _returnvalue_2 (Game|GetCurrentLevelName true))
    (Variables|/Game/BluePrints/GmaeInstance_BP.GmaeInstance_BP_C|SetbeforeLevelName _asgmae_instance_bp (Utilities|String|StringToName _returnvalue_2))
    (bind _returnvalue_3 (UserInterface|CreateWidget "/Game/BluePrints/UMG/FadeWidget_BP.FadeWidget_BP_C" 0 false))
    (UserInterface|Viewport|AddtoViewport _returnvalue_3 0)
    (Utilities|FlowControl|Sequence
      (:then_0
        (Game|LoadStreamLevel(byName) "Loading" true))
      (:then_1
        (Utilities|FlowControl|Delay 0.5)
        (Game|OpenLevel(byName) "Loading")))))

(fn ConstructionScript)