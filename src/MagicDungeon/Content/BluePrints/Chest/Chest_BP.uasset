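; Treasure chest Blueprint that opens on an action event from Marisa and yields a Crystal, guarded by a check on the stored spawn reference.
; The event removes the widget, sets Open on the chest's AnimBP, then spawns the Crystal at the chest with its CrystalNum after a short delay.
; An Up timeline lifts the Crystal along Z, then after a pause calls GetMessage on it with Marisa.
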(event EventBeginPlay
  (Variables|Default|SetmyABP (.AsChest%20ABP (Utilities|Casting|CastToChest_ABP (Components|SkeletalMesh|GetAnimInstance (Variables|Default|GetChest))))))

(event EventActorBeginOverlap
  (params (OtherActor :type Actor%20Object%20Reference)))

(event EventTick
  (params (DeltaSeconds :type Float%20%28single-precision%29)))

(event EventActionEvent
  (params (marisa :type Marisa%20BP%20Object%20Reference))
  (if (== (Variables|Default|Getspawn) 0)
    (CallFunction|RemoveWidget)
    (Variables|Default|Setmarisa marisa)
    (Variables|/Game/BluePrints/Chest/Chest_ABP.Chest_ABP_C|Setopen (Variables|Default|GetmyABP) true)
    (Utilities|FlowControl|Delay 0.2)
    (bind _returnvalue (Game|SpawnActorfromClass "/Game/BluePrints/Crystal/Crystal.Crystal_C" (Transformation|GetActorTransform) "Undefined" 0 (Variables|Default|GetcrystalNum) 0))
    (Variables|Default|Setspawn _returnvalue)
    (bind _value (Timeline|up Play)
      (:Update
        (Transformation|AddActorWorldOffset (Variables|Default|Getspawn) (Math|Vector|MakeVector 0.0 0.0 _value)))
      (:Finished
        (Utilities|FlowControl|Delay 1.5)
        (Class|ChestInterface|Get(Message) (Variables|Default|Getspawn) (Variables|Default|Getmarisa))))))

(fn ConstructionScript)