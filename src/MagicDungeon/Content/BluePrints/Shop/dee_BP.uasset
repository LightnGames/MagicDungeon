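; Dee is a shop NPC actor who offers Marisa magic upgrades for crystals through a scripted conversation.
; ActionEvent pauses Marisa, moves input to Dee, creates the talk widget and eases Marisa's camera to a shop viewpoint.
; The attack key pages dialogue; page 5 opens the shop widget and blocks paging until FinishCall.
; When dialogue ends, the battle UI updates and a second timeline restores the camera before control returns to Marisa.
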(event EventBeginPlay)

(event EventActorBeginOverlap
  (params (OtherActor :type Actor%20Object%20Reference)))

(event EventTick
  (params (DeltaSeconds :type Float%20%28single-precision%29)))

(event EventFinishCall
  (Default|NextPage (Variables|Default|GettalkWidget))
  (Variables|Default|SetstopCall false))

(event EventActionEvent
  (params (marisa :type Marisa%20BP%20Object%20Reference))
  (|初期化＆Widgt生成 marisa)
  (Variables|Default|SetdefaultCameraTransform (Transformation|GetWorldTransform (Variables|/Game/BluePrints/Marisa_BP.Marisa_BP_C|GetCamera (Variables|Default|Getmarisa))))
  (bind _fade (Timeline|CameraIn PlayFromStart)
    (:Update
      (Transformation|SetWorldTransform (Variables|/Game/BluePrints/Marisa_BP.Marisa_BP_C|GetCamera (Variables|Default|Getmarisa)) (Math|Interpolation|Ease "EaseInOut" _fade (Variables|Default|GetdefaultCameraTransform) (Transformation|GetWorldTransform (Variables|Default|GetCameraPosition)) 2.0) false false))
    (:Finished
      (Default|NextPage (Variables|Default|GettalkWidget)))))

(event Input|ActionEvents|InputActionattack
  (params (Key :type Key%20Structure :default "AnyKey"))
  (bind _returnvalue (Game|GetPlayerController 0))
  (bind _marisa (Variables|Default|Getmarisa))
  (:Pressed
    (if (not (Variables|Default|GetstopCall))
      (bind (_end _nowpage) (Default|NextPage (Variables|Default|GettalkWidget)))
      (if (== _nowpage 5)
        (if (== (Variables|Default|GetshopWidget) 0)
          (bind _returnvalue_2 (UserInterface|CreateWidget "/Game/BluePrints/Shop/ShopWidget_BP.ShopWidget_BP_C" 0 (Variables|Default|Getmarisa) self))
          (UserInterface|Viewport|AddtoViewport _returnvalue_2 0)
          (Variables|Default|SetshopWidget _returnvalue_2)
          (Variables|Default|SetstopCall true))
        (elif _end
          (Default|FinishCall (Variables|Default|GettalkWidget))
          (Default|UpdateData (Variables|/Game/BluePrints/ButtleGameMode_BP.ButtleGameMode_BP_C|GetbuttleUI (.AsButtle%20Game%20Mode%20BP (Utilities|Casting|CastToButtleGameMode_BP (Game|GetGameMode)))))
          (bind _fade (Timeline|タイムライン_0 PlayFromStart)
            (:Update
              (Transformation|SetWorldTransform (Variables|/Game/BluePrints/Marisa_BP.Marisa_BP_C|GetCamera (Variables|Default|Getmarisa)) (Math|Interpolation|Ease "EaseInOut" _fade (Transformation|GetWorldTransform (Variables|Default|GetCameraPosition)) (Variables|Default|GetdefaultCameraTransform) 2.0) false false))
            (:Finished
              (Variables|/Game/BluePrints/Marisa_BP.Marisa_BP_C|Setpause _marisa false)
              (Input|EnableInput _marisa _returnvalue)
              (Input|DisableInput _returnvalue)
              (Variables|Default|SetshopWidget 0))))))))

(fn ConstructionScript)