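; Base talk NPC for the shop that runs a paged dialogue with Marisa when ActionEvent fires.
; It pauses Marisa, takes over input, creates TalkWidget_BP from TalkDatas and eases her camera to CameraPosition.
; Attack advances pages through an empty CallBackNextPage hook, with StopCall blocking advance until FinishCall resumes it.
; The last page closes the talk, refreshes battle UI, eases the camera back and unpauses Marisa.
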(event EventFinishCall
  (Default|NextPage (Variables|Default|GettalkWidget))
  (CallFunction|ShowWidget)
  (Variables|Default|SetstopCall false))

(event EventActionEvent
  (params (marisa :type Marisa%20BP%20Object%20Reference))
  (|初期化＆Widgt生成_2 marisa)
  (CallFunction|RemoveWidget)
  (Variables|Default|SetdefaultCameraTransform (Transformation|GetWorldTransform (Variables|/Game/BluePrints/Marisa/Marisa_BP.Marisa_BP_C|GetCamera (Variables|Default|Getmarisa))))
  (bind _fade (Timeline|タイムライン_0 PlayFromStart)
    (:Update
      (Transformation|SetWorldTransform (Variables|/Game/BluePrints/Marisa/Marisa_BP.Marisa_BP_C|GetCamera (Variables|Default|Getmarisa)) (Math|Interpolation|Ease "EaseInOut" _fade (Variables|Default|GetdefaultCameraTransform) (Transformation|GetWorldTransform (Variables|Default|GetCameraPosition)) 2.0) false false))
    (:Finished
      (Default|NextPage (Variables|Default|GettalkWidget)))))

(event Input|ActionEvents|InputActionattack
  (params (Key :type Key%20Structure :default "AnyKey"))
  (bind _returnvalue (Game|GetPlayerController 0))
  (:Pressed
    (if (not (Variables|Default|GetstopCall))
      (bind (_end _nowpage) (Default|NextPage (Variables|Default|GettalkWidget)))
      (CallFunction|CallBackNextPage _end _nowpage)
      (if _end
        (Default|FinishCall (Variables|Default|GettalkWidget))
        (Default|UpdateData (Variables|/Game/BluePrints/ButtleGameMode_BP.ButtleGameMode_BP_C|GetbuttleUI (.AsButtle%20Game%20Mode%20BP (Utilities|Casting|CastToButtleGameMode_BP (Game|GetGameMode)))))
        (bind _fade (Timeline|タイムライン_1 PlayFromStart)
          (:Update
            (Transformation|SetWorldTransform (Variables|/Game/BluePrints/Marisa/Marisa_BP.Marisa_BP_C|GetCamera (Variables|Default|Getmarisa)) (Math|Interpolation|Ease "EaseInOut" _fade (Transformation|GetWorldTransform (Variables|Default|GetCameraPosition)) (Variables|Default|GetdefaultCameraTransform) 2.0) false false))
          (:Finished
            (Variables|/Game/BluePrints/Marisa/Marisa_BP.Marisa_BP_C|Setpause (Variables|Default|Getmarisa) false)
            (Input|EnableInput _returnvalue)
            (Input|DisableInput _returnvalue)))))))

(fn ConstructionScript
  (|CallParentFunction))

(fn CallBackNextPage
  (params (end :type Boolean) (nowPage :type Integer)))