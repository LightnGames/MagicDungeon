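; Battle game mode that sets up the battle HUD, the player character Marisa and a magic inventory screen.
; On BeginPlay it shows ButtoleUI, passes itself to Marisa, creates Enventry_BP with Marisa, MagicDatas and the HUD, then initializes Marisa.
; The inventory is finished and hidden right after creation, and the enventry input toggles the same instance through a FlipFlop, calling Finish before each removal.
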(event EventBeginPlay
  (Input|EnableInput (Game|GetPlayerController 0))
  (bind _returnvalue (UserInterface|CreateWidget "/Game/BluePrints/UMG/ButtoleUI.ButtoleUI_C"))
  (UserInterface|Viewport|AddtoViewport _returnvalue 0)
  (bind _output_get (Variables|Default|SetbuttleUI _returnvalue))
  (|プレイヤー取得&初期化_2)
  (|EnventryWidget追加 _output_get)
  (Default|Initialize (Variables|Default|Getmarisa)))

(event EventTick
  (params (DeltaSeconds :type Float%20%28single-precision%29)))

(event Input|ActionEvents|InputActionenventry
  (params (Key :type Key%20Structure :default "AnyKey"))
  (bind _enventry (Variables|Default|Getenventry))
  (:Pressed
    (Utilities|FlowControl|FlipFlop
      (:A
        (UserInterface|Viewport|AddtoViewport _enventry 0))
      (:B
        (Default|Finish _enventry)
        (Widget|RemovefromParent _enventry)))))

(fn ConstructionScript)