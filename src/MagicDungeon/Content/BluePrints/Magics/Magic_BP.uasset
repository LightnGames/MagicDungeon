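; Base magic actor for spells cast by the player (Marisa) or enemies, destroying itself once DieCheckStart is set and its particle is gone.
; Hit skips "NoBody" components, damages the opposing side using MyData or override data, and shows a damage widget, returning true only for enemy hits.
; Damage varies randomly by ±10%, rolled separately for application and display.
; SwitchCollision toggles collision by moving components out of range, and MagicFinish fires FinishCall.
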(event EventBeginPlay)

(event EventActorBeginOverlap
  (params (OtherActor :type Actor%20Object%20Reference)))

(event EventTick
  (params (DeltaSeconds :type Float%20%28single-precision%29))
  (if (not (or (and (Utilities|IsValid (Variables|Default|GetmyParticle)) (!= (Variables|Default|GetmyParticle) 0)) (not (Variables|Default|GetdieCheckStart))))
    (Variables|Default|SetmyParticle 0)
    (Actor|DestroyActor)))

(fn ConstructionScript)

(fn MagicFinish
  (CallFunction|FinishCall))

(fn Hit
  (params (target :type Actor%20Object%20Reference) (component :type Scene%20Component%20Object%20Reference) (overrideData :type Magic%20Datas%20Structure))
  (bind _damage (Utilities|Struct|BreakMagicDatas overrideData))
  (bind _returnvalue (Math|Random|RandomFloatinRange -1.0 1.0))
  (bind _mydata (Variables|Default|GetmyData))
  (bind _returnvalue_2 (== _damage 0))
  (bind _returnvalue_3 (select _returnvalue_2 _mydata overrideData))
  (bind _damage_2 (Utilities|Struct|BreakMagicDatas _returnvalue_3))
  (bind _returnvalue_4 (Math|Conversions|ToFloat(Integer) _damage_2))
  (bind _returnvalue_5 (* _returnvalue_4 0.1 _returnvalue))
  (bind _returnvalue_6 (Math|Float|Truncate _returnvalue_5))
  (bind _returnvalue_7 (+ _damage_2 _returnvalue_6))
  (bind _returnvalue_8 (Math|Conversions|ToFloat(Integer) _returnvalue_7))
  (if (== component 0)
    (if (Variables|Default|GetplayerSIde) :!label _label
      (bind _asenemy (Utilities|Casting|CastToEnemy target)
        (:then
          (Game|Damage|ApplyDamage _asenemy _returnvalue_8 0 0)
          (Utilities|DisplayWidget _returnvalue_7 _asenemy)
          (Variables|/Game/BluePrints/Enemys/Enemy.Enemy_C|Setmarisa _asenemy (Variables|Default|Getmarisa))
          (return true))
        (:CastFailed
          _))
      (else
        (bind _asmarisa_bp (Utilities|Casting|CastToMarisa_BP target)
          (:then
            (Game|Damage|ApplyDamage _asmarisa_bp _returnvalue_8 0 0)
            (Utilities|DisplayWidget _returnvalue_7 _asmarisa_bp))
          (:CastFailed
            _))))
    (return false)
    (elif (not (Components|ComponentHasTag component "NoBody"))
      (goto _label))))

(fn SwitchCollision
  (params (set :type Boolean) (target :type Scene%20Component%20Object%20Reference))
  (if set
    (Transformation|SetRelativeLocation target "0, 0,0.000000" false false)
    (else
      (Transformation|SetRelativeLocation target "0, 0,-1000.000000" false false))))