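; Small tornado spell actor that moves toward actors caught in its sphere and hits each in turn.
; On spawn it attaches the tornado particle, scales up, draws a debug sphere and switches sphere collision off after a short delay.
; Overlapping actors are queued as targets.
; Tick steps a fixed distance per frame toward the first, unscaled by delta time, then calls Hit and dequeues it when very close.
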(event OnComponentBeginOverlap(Sphere)
  (params (OtherActor :type Actor%20Object%20Reference) (OtherComp :type Primitive%20Component%20Object%20Reference) (OtherBodyIndex :type Integer) (bFromSweep :type Boolean) (SweepResult :type Hit%20Result%20Structure%20%28by%20ref%29))
  (Utilities|Array|Add (Variables|Default|Gettargets) OtherActor))

(event EventBeginPlay
  (bind _sphere (Variables|Default|GetSphere))
  (|CallParentFunction)
  (Rendering|Debug|DrawDebugSphere (Transformation|GetWorldLocation _sphere) (Variables|/Script/Engine.SphereComponent|GetSphereRadius _sphere) 12 "(R=1.000000,G=1.000000,B=1.000000,A=1.000000)" 1e+01)
  (bind _returnvalue (Effects|SpawnEmitterAttached "/Game/KYmagicFX05/Particles/once/P_tornadeLv1.P_tornadeLv1" (Variables|Default|GetDefaultSceneRoot) "None" "0, 0, 0" "0, 0,0.000000"))
  (Transformation|SetActorScale3D "1.500000,1.500000,1.500000")
  (Variables|Default|SetmyParticle _returnvalue)
  (Utilities|FlowControl|Delay 0.5)
  (CallFunction|SwitchCollision false (Variables|Default|GetSphere)))

(event EventTick
  (params (DeltaSeconds :type Float%20%28single-precision%29))
  (bind _returnvalue (Transformation|GetActorLocation))
  (bind _targets (Variables|Default|Gettargets))
  (bind _targets_2 (Variables|Default|Gettargets))
  (bind _item (Utilities|Array|Get(acopy) _targets))
  (bind _returnvalue_2 (Transformation|GetActorLocation _item))
  (bind _returnvalue_3 (- _returnvalue_2 _returnvalue))
  (|CallParentFunction DeltaSeconds)
  (if (> (Utilities|Array|Length (Variables|Default|Gettargets)) 0)
    (Transformation|SetActorLocation (+ (* (Math|Vector|Normalize _returnvalue_3) 3) _returnvalue) false false)
    (if (< (Math|Vector|VectorLength _returnvalue_3) 5.0)
      (CallFunction|Hit (Utilities|Array|Get(acopy) _targets_2))
      (Utilities|Array|RemoveIndex _targets_2))))

(fn ConstructionScript
  (|CallParentFunction))