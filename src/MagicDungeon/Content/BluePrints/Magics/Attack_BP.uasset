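; Magic attack Blueprint that briefly opens a sphere hitbox and, on a successful hit, changes Marisa's MP by the negated damage value.
; BeginPlay applies optional scale, damage and timing overrides, waits for the hit time, then attaches a sonic slash particle and enables collision.
; After a short window it disables collision and sets DieCheckStart; a debug sphere draws the hit area.
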(event OnComponentBeginOverlap(Sphere)
  (params (OtherActor :type Actor%20Object%20Reference) (OtherComp :type Primitive%20Component%20Object%20Reference) (OtherBodyIndex :type Integer) (bFromSweep :type Boolean) (SweepResult :type Hit%20Result%20Structure%20%28by%20ref%29))
  (bind _value (CallFunction|Hit OtherActor OtherComp))
  (if _value
    (Default|MPUpDown (Variables|Default|Getmarisa) (* (.damage (Variables|Default|GetmyData)) -1))))

(event EventBeginPlay
  (bind _overrideattackpoint (Variables|Default|GetoverrideAttackPoint))
  (bind _overridescale (Variables|Default|GetoverrideScale))
  (bind _sphere (Variables|Default|GetSphere))
  (bind _overridehittime (Variables|Default|GetoverrideHitTime))
  (bind _returnvalue (== _overridescale 0.0))
  (bind _returnvalue_2 (select _returnvalue 1.0 _overridescale))
  (|CallParentFunction)
  (Transformation|SetRelativeScale3D (Variables|Default|GetSphere) (Math|Vector|MakeVector _returnvalue_2 _returnvalue_2 _returnvalue_2))
  (if (== _overrideattackpoint 0)
    _
    (else
      (Variables|Default|SetmyData (Utilities|Struct|MakeMagicDatas "" 0 _overrideattackpoint 0 0.0 0 0 0 0 0 0.0 "" (Utilities|Array|MakeArray "")))))
  (if (== _overridehittime 0.0)
    _
    (else
      (Variables|Default|SethitTime _overridehittime)))
  (Collision|SetCollisionEnabled (Variables|Default|GetSphere) "NoCollision")
  (Utilities|FlowControl|Delay (Variables|Default|GethitTime))
  (bind _returnvalue_3 (Effects|SpawnEmitterAttached "/Game/KYmagicFX05/Particles/P_sonicSlash.P_sonicSlash" (Variables|Default|GetScene) "None"))
  (Variables|Default|SetmyParticle _returnvalue_3)
  (Collision|SetCollisionEnabled (Variables|Default|GetSphere) "QueryAndPhysics")
  (Rendering|Debug|DrawDebugSphere (Transformation|GetWorldLocation _sphere) (Variables|/Script/Engine.SphereComponent|GetSphereRadius _sphere) 12 "(R=1.000000,G=1.000000,B=1.000000,A=1.000000)" 3.0)
  (Utilities|FlowControl|Delay (Variables|Default|GetdestroyCollisionTime))
  (Collision|SetCollisionEnabled (Variables|Default|GetSphere) "NoCollision")
  (Variables|Default|SetdieCheckStart true))

(event EventTick
  (params (DeltaSeconds :type Float%20%28single-precision%29))
  (|CallParentFunction 0.0))

(fn ConstructionScript
  (|CallParentFunction))