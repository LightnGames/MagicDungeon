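; Recovery magic actor that applies its data-driven damage value to Marisa, named and styled as a recovery spell.
; On BeginPlay it attaches the recovery particle effect to Marisa's mesh and starts the DistanceCheck timeline.
; Each timeline event calls DamageOverlap on Marisa as player-side, passing the full value while Marisa is within a short radius of the actor and half otherwise.
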(event EventBeginPlay
  (bind _mydata (Variables|Default|GetmyData))
  (|CallParentFunction)
  (Effects|SpawnEmitterAttached "/Game/KYmagicFX05/Particles/once/P_recovery.P_recovery" (Variables|/Script/Engine.Character|GetMesh (Variables|Default|Getmarisa)) "None")
  (Timeline|DistanceCheck Play
    (:event
      (CallFunction|DamageOverlap (Variables|Default|Getmarisa) (select (< (Math|Vector|VectorLength (- (Transformation|GetActorLocation (Variables|Default|Getmarisa)) (Transformation|GetActorLocation))) 2e+02) (.damage _mydata) (/ (.damage _mydata) 2)) true false))))

(fn ConstructionScript
  (|CallParentFunction))