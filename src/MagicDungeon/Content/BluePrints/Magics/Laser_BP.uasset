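; Laser magic attack actor that damages actors inside a sphere during a timed collision window.
; On BeginPlay it attaches an aqua splash particle, enables sphere collision after HitTime, disables it after DestroyCollisionTime, then sets DieCheckStart and draws a debug sphere.
; Sphere overlap starts the DamageCount timeline, whose event track calls Hit on the overlapping actor; ending the overlap stops it.
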(event OnComponentBeginOverlap(Sphere)
  (params (OtherActor :type Actor%20Object%20Reference) (OtherComp :type Primitive%20Component%20Object%20Reference) (OtherBodyIndex :type Integer) (bFromSweep :type Boolean) (SweepResult :type Hit%20Result%20Structure%20%28by%20ref%29))
  (Timeline|DamageCount PlayFromStart
    (:event
      (CallFunction|Hit OtherActor OtherComp))))

(event OnComponentEndOverlap(Sphere)
  (params (OtherActor :type Actor%20Object%20Reference) (OtherComp :type Primitive%20Component%20Object%20Reference) (OtherBodyIndex :type Integer))
  (Timeline|DamageCount Stop
    (:event
      (CallFunction|Hit (stale OnComponentBeginOverlap(Sphere) OtherActor) (stale OnComponentBeginOverlap(Sphere) OtherComp)))))

(event EventBeginPlay
  (bind _sphere (Variables|Default|GetSphere))
  (|CallParentFunction)
  (CallFunction|SwitchCollision false (Variables|Default|GetSphere))
  (bind _returnvalue (Effects|SpawnEmitterAttached "/Game/KYmagicFX05/Particles/P_aquaSplash.P_aquaSplash" (Variables|Default|GetDefaultSceneRoot) "None" (Variables|/Script/Engine.SceneComponent|GetRelativeLocation (Variables|Default|GetParticleLocation)) "90,90,0.0"))
  (Variables|Default|SetmyParticle _returnvalue)
  (Utilities|FlowControl|Delay (Variables|Default|GethitTime))
  (CallFunction|SwitchCollision true (Variables|Default|GetSphere))
  (Utilities|FlowControl|Delay (Variables|Default|GetdestroyCollisionTime))
  (CallFunction|SwitchCollision false _sphere)
  (Variables|Default|SetdieCheckStart true)
  (Rendering|Debug|DrawDebugSphere (Transformation|GetWorldLocation _sphere) (Variables|/Script/Engine.SphereComponent|GetSphereRadius _sphere) 12 "(R=1.000000,G=0.000000,B=0.037874,A=1.000000)" 3.0))

(event EventActorBeginOverlap
  (params (OtherActor :type Actor%20Object%20Reference)))

(event EventTick
  (params (DeltaSeconds :type Float%20%28single-precision%29))
  (|CallParentFunction 0.0))

(fn ConstructionScript
  (|CallParentFunction))