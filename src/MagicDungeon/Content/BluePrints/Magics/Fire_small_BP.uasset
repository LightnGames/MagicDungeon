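; Small fire magic Blueprint that hits overlapping actors during a timed collision window, built on a parent class.
; BeginPlay attaches the P_rayLv1 particle, enables the sphere collision after HitTime, then disables it after DestroyCollisionTime and sets DieCheckStart.
; Sphere overlaps send a "Fire" gimmick event to the other actor and call Hit on it.
; A debug sphere is drawn at the collision volume once the window closes.
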(event OnComponentBeginOverlap(Sphere)
  (params (OtherActor :type Actor%20Object%20Reference) (OtherComp :type Primitive%20Component%20Object%20Reference) (OtherBodyIndex :type Integer) (bFromSweep :type Boolean) (SweepResult :type Hit%20Result%20Structure%20%28by%20ref%29))
  (Class|StageGimicInterface|GimicEvent(Message) OtherActor "Fire" 0.0)
  (CallFunction|Hit OtherActor OtherComp))

(event EventBeginPlay
  (bind _sphere (Variables|Default|GetSphere))
  (|CallParentFunction)
  (CallFunction|SwitchCollision false (Variables|Default|GetSphere))
  (bind _returnvalue (Effects|SpawnEmitterAttached "/Game/KYmagicFX05/Particles/P_rayLv1.P_rayLv1" (Variables|Default|GetDefaultSceneRoot) "None" (Math|Vector|MakeVector 0.0 0.0 (Variables|Default|GetEmitterYOffset)) "0, 0,0.000000"))
  (Variables|Default|SetmyParticle _returnvalue)
  (Utilities|FlowControl|Delay (Variables|Default|GethitTime))
  (CallFunction|SwitchCollision true (Variables|Default|GetSphere))
  (Utilities|FlowControl|Delay (Variables|Default|GetdestroyCollisionTime))
  (CallFunction|SwitchCollision false (Variables|Default|GetSphere))
  (Variables|Default|SetdieCheckStart true)
  (Rendering|Debug|DrawDebugSphere (Transformation|GetWorldLocation _sphere) (Variables|/Script/Engine.SphereComponent|GetSphereRadius _sphere) 12 "(R=1.000000,G=1.000000,B=1.000000,A=1.000000)" 3.0))

(event EventTick
  (params (DeltaSeconds :type Float%20%28single-precision%29)))

(fn ConstructionScript
  (|CallParentFunction))