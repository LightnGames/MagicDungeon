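; Snake enemy Blueprint that drives its animation Blueprint from gameplay events.
; On BeginPlay it caches the mesh's Snake_ABP instance and registers itself as that instance's Enemy.
; The Walking event sets the Run flag and plays the Checking timeline, clearing Run when it finishes.
; DieOverride sets the Die flag, while Tick only calls the parent implementation.
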(event EventBeginPlay
  (|CallParentFunction)
  (bind _output_get (Variables|Default|SetmyABP (.AsSnake%20ABP (Utilities|Casting|CastToSnake_ABP (Components|SkeletalMesh|GetAnimInstance (Variables|Character|GetMesh))))))
  (Variables|/Game/BluePrints/Enemys/Snake/Snake_ABP.Snake_ABP_C|Setenemy _output_get self))

(event EventActorBeginOverlap
  (params (OtherActor :type Actor%20Object%20Reference)))

(event EventTick
  (params (DeltaSeconds :type Float%20%28single-precision%29))
  (|CallParentFunction DeltaSeconds))

(event EventDieOverride
  (Variables|/Game/BluePrints/Enemys/Snake/Snake_ABP.Snake_ABP_C|Setdie (Variables|Default|GetmyABP) true))

(event EventWalking
  (bind _myabp (Variables|Default|GetmyABP))
  (Variables|/Game/BluePrints/Enemys/Snake/Snake_ABP.Snake_ABP_C|Setrun _myabp true)
  (Timeline|checking PlayFromStart
    (:Finished
      (Variables|/Game/BluePrints/Enemys/Snake/Snake_ABP.Snake_ABP_C|Setrun _myabp false))))

(fn ConstructionScript)