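; Spider enemy Blueprint that adds animation and attack behavior on top of its parent class.
; Walk and turn events set the Walking flag in Spider_ABP while alive, clearing it when the CheckWalk timeline finishes.
; Attack overrides and Box overlaps with Marisa_BP trigger the attack animation and spawn an enemy-side EnemyAttack_BP ahead, with different scale and hit-time overrides.
; The death override sets the Die flag.
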(event OnComponentBeginOverlap(Box)
  (params (OtherActor :type Actor%20Object%20Reference) (OtherComp :type Primitive%20Component%20Object%20Reference) (OtherBodyIndex :type Integer) (bFromSweep :type Boolean) (SweepResult :type Hit%20Result%20Structure%20%28by%20ref%29))
  (bind _returnvalue (Transformation|GetActorRotation))
  (Utilities|Casting|CastToMarisa_BP OtherActor)
  (Variables|/Game/BluePrints/Enemys/Spider/Spider_ABP.Spider_ABP_C|Setattack (Variables|Default|GetmyABP) true)
  (Game|SpawnActorfromClass "/Game/BluePrints/Magics/EnemyAttack_BP.EnemyAttack_BP_C" (Math|Transform|MakeTransform (+ (Transformation|GetActorLocation) (* (Math|Vector|GetForwardVector _returnvalue) 1e+02)) _returnvalue "1,1,1") "Undefined" 0 1.5 0.0 (Variables|Default|GetbaseAttackPoint) 0 false))

(event EventWalking
  (if (> (Variables|Default|Gethp) 0)
    (Variables|/Game/BluePrints/Enemys/Spider/Spider_ABP.Spider_ABP_C|Setwalking (Variables|Default|GetmyABP) true)
    (Timeline|CheckWalk PlayFromStart
      (:Finished
        _)))
  (Variables|/Game/BluePrints/Enemys/Spider/Spider_ABP.Spider_ABP_C|Setwalking (Variables|Default|GetmyABP) false))

(event EventBeginPlay
  (|CallParentFunction)
  (bind _output_get (Variables|Default|SetmyABP (.AsSpider%20ABP (Utilities|Casting|CastToSpider_ABP (Components|SkeletalMesh|GetAnimInstance (Variables|Character|GetMesh))))))
  (Variables|/Game/BluePrints/Enemys/Spider/Spider_ABP.Spider_ABP_C|Setenemy _output_get self))

(event EventTick
  (params (DeltaSeconds :type Float%20%28single-precision%29))
  (|CallParentFunction DeltaSeconds))

(event EventAttackOverride
  (params (actor :type Actor%20Object%20Reference))
  (bind _returnvalue (Transformation|GetActorRotation))
  (Variables|Default|SetnowTarget actor)
  (Variables|/Game/BluePrints/Enemys/Spider/Spider_ABP.Spider_ABP_C|Setattack (Variables|Default|GetmyABP) true)
  (Game|SpawnActorfromClass "/Game/BluePrints/Magics/EnemyAttack_BP.EnemyAttack_BP_C" (Math|Transform|MakeTransform (+ (Transformation|GetActorLocation) (* (Math|Vector|GetForwardVector _returnvalue) 1e+02)) _returnvalue "1,1,1") "Undefined" 0 0.0 0.5 (Variables|Default|GetbaseAttackPoint) 0 false))

(event EventDieOverride
  (Variables|/Game/BluePrints/Enemys/Spider/Spider_ABP.Spider_ABP_C|Setdie (Variables|Default|GetmyABP) true))

(event EventTern
  (if (> (Variables|Default|Gethp) 0)
    (Variables|/Game/BluePrints/Enemys/Spider/Spider_ABP.Spider_ABP_C|Setwalking (Variables|Default|GetmyABP) true)
    (Timeline|CheckWalk PlayFromStart
      (:Finished
        _)))
  (Variables|/Game/BluePrints/Enemys/Spider/Spider_ABP.Spider_ABP_C|Setwalking (Variables|Default|GetmyABP) false))

(fn ConstructionScript
  (|CallParentFunction))