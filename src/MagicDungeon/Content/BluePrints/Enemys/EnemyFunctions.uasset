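; Enemy AI helper functions with a check for whether an enemy can reach a goal actor, by name the player, in a straight navmesh path.
; When the goal is within the given length, a navigation raycast runs to it and reports success only if the hit location exactly matches the goal's location.
; Out-of-range goals return false with the Through flag set, and each raycast draws a debug line.
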(fn CheckCanArrivePlayer
  (params (enemuAI :type AI%20Controller%20Object%20Reference) (enemy :type Actor%20Object%20Reference) (goal :type Actor%20Object%20Reference) (length :type Float%20%28single-precision%29))
  (bind _returnvalue (Transformation|GetActorLocation enemy))
  (bind _returnvalue_2 (Transformation|GetActorLocation goal))
  (if (< (Math|Vector|VectorLength (- _returnvalue _returnvalue_2)) length)
    (bind _hitlocation (Class|NavigationSystem|NavigationRaycast enemuAI _returnvalue _returnvalue_2))
    (Rendering|Debug|DrawDebugLine 0 _returnvalue _hitlocation "(R=0.000000,G=0.066276,B=1.000000,A=1.000000)" 1.0 1.0)
    (return (== (Math|Vector|VectorLength (- _hitlocation _returnvalue_2)) 0.0) false)
    (else
      (return false true))))