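; DropStone_BP is a destructible falling rock in the StoneDemon enemy folder that damages the player character, Marisa_BP.
; On BeginPlay it traces downward and spawns a red, scaled-up EnemyDecal_BP at the trace hit location.
; The first component hit sets collision to physics-only and latches a Damaged flag, applying damage and a damage widget only if it struck Marisa.
; When the mesh fractures, the actor destroys itself after a short delay.
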(event OnComponentFracture(Rock_03_DM)
  (params (HitPoint :type Vector%20%28by%20ref%29 :default "0, 0, 0") (HitDirection :type Vector%20%28by%20ref%29 :default "0, 0, 0"))
  (Utilities|FlowControl|Delay 5.0)
  (Actor|DestroyActor))

(event OnComponentHit(Rock_03_DM)
  (params (OtherActor :type Actor%20Object%20Reference) (OtherComp :type Primitive%20Component%20Object%20Reference) (NormalImpulse :type Vector :default "0, 0, 0") (Hit :type Hit%20Result%20Structure%20%28by%20ref%29))
  (bind _damage (Variables|Default|Getdamage))
  (Collision|SetCollisionEnabled (Variables|Default|GetRock_03_DM) "PhysicsOnly")
  (bind _asmarisa_bp (Utilities|Casting|CastToMarisa_BP OtherActor)
    (:then
      (if (not (Variables|Default|Getdamaged))
        (CallFunction|DisplayDamageWidget _asmarisa_bp _damage false false)
        (Game|Damage|ApplyDamage _asmarisa_bp (Math|Conversions|ToFloat(Integer) _damage) 0 0)
        (Variables|Default|Setdamaged true :!label _label)))
    (:CastFailed
      (goto _label))))

(event EventBeginPlay
  (bind _returnvalue (Transformation|GetActorLocation))
  (bind _returnvalue_2 (Transformation|GetActorRotation))
  (bind _returnvalue_3 (Math|Conversions|ToFloat(Integer) 2))
  (bind _returnvalue_4 (Math|Vector|GetUpVector _returnvalue_2))
  (bind _outhit (Collision|LineTraceByChannel (+ _returnvalue (* _returnvalue_4 -200)) (+ _returnvalue (* _returnvalue_4 -1000)) "TraceTypeQuery1" false 0 "ForDuration"))
  (Game|SpawnActorfromClass "/Game/BluePrints/Enemys/StoneDemon/EnemyDecal_BP.EnemyDecal_BP_C" (Math|Transform|MakeTransform (.Location (Collision|BreakHitResult _outhit)) "0, 0, 0" (Math|Vector|MakeVector _returnvalue_3 _returnvalue_3 _returnvalue_3)) "Undefined" 0 (Utilities|Struct|MakeLinearColor 1.0 0.0 0.060141 0.0) 0))

(event EventTick
  (params (DeltaSeconds :type Float%20%28single-precision%29)))

(fn ConstructionScript)