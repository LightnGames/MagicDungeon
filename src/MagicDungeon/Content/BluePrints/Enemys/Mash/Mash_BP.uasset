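; Mash_BP is an enemy Blueprint that drives its Mash_ABP animation instance through attack, walk and death flags.
; ThrowAttack sets the attack flag and spawns a FireBall ahead of the actor, passing speed and base attack damage.
; Tern and Walking share one path that, while Hp is above zero, holds the walk flag until a timeline finishes.
; DieOverride sets the death flag.
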(event EventTern
  (if (> (Variables|Default|Gethp) 0)
    (Variables|/Game/BluePrints/Enemys/Mash/Mash_ABP.Mash_ABP_C|Setwalk (Variables|Default|GetmyABP) true)
    (Timeline|タイムライン_0 PlayFromStart
      (:Finished
        _)))
  (Variables|/Game/BluePrints/Enemys/Mash/Mash_ABP.Mash_ABP_C|Setwalk (Variables|Default|GetmyABP) false))

(event EventWalking
  (if (> (Variables|Default|Gethp) 0)
    (Variables|/Game/BluePrints/Enemys/Mash/Mash_ABP.Mash_ABP_C|Setwalk (Variables|Default|GetmyABP) true)
    (Timeline|タイムライン_0 PlayFromStart
      (:Finished
        _)))
  (Variables|/Game/BluePrints/Enemys/Mash/Mash_ABP.Mash_ABP_C|Setwalk (Variables|Default|GetmyABP) false))

(event EventBeginPlay
  (|CallParentFunction)
  (bind _output_get (Variables|Default|SetmyABP (.AsMash%20ABP (Utilities|Casting|CastToMash_ABP (Components|SkeletalMesh|GetAnimInstance (Variables|Character|GetMesh))))))
  (Variables|/Game/BluePrints/Enemys/Mash/Mash_ABP.Mash_ABP_C|Setenemy _output_get self))

(event EventActorBeginOverlap
  (params (OtherActor :type Actor%20Object%20Reference)))

(event EventTick
  (params (DeltaSeconds :type Float%20%28single-precision%29))
  (|CallParentFunction DeltaSeconds))

(event EventDieOverride
  (Variables|/Game/BluePrints/Enemys/Mash/Mash_ABP.Mash_ABP_C|Setdie (Variables|Default|GetmyABP) true))

(event EventThrowAttack
  (params (forwardValue :type Float%20%28single-precision%29) (speed :type Float%20%28single-precision%29))
  (bind _returnvalue (Transformation|GetActorRotation))
  (Variables|/Game/BluePrints/Enemys/Mash/Mash_ABP.Mash_ABP_C|Setattack (Variables|Default|GetmyABP) true)
  (Game|SpawnActorfromClass "/Game/BluePrints/Enemys/Mash/FireBall.FireBall_C" (Math|Transform|MakeTransform (+ (* (Math|Vector|GetForwardVector _returnvalue) forwardValue) (Transformation|GetActorLocation)) _returnvalue "1,1,1") "Undefined" 0 speed (Math|Conversions|ToFloat(Integer) (Variables|Default|GetbaseAttackPoint))))

(fn ConstructionScript)