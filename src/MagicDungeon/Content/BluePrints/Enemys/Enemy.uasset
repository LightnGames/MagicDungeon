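; Base enemy Blueprint that tracks HP and grants EXP to Marisa when killed.
; Taking damage spawns an explosion effect, lowers HP and shows an on-screen status widget, which Tick updates and removes after ten seconds without further hits.
; Death and attack behavior go through empty DieOverride and AttackOverride hooks; death does not itself call DestroyEnemy, which is a separate function.
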(event EventBeginPlay
  (Variables|System|Sethp (Variables|Default|GetmaxHP)))

(event EventActorBeginOverlap
  (params (OtherActor :type Actor%20Object%20Reference)))

(event EventTick
  (params (DeltaSeconds :type Float%20%28single-precision%29))
  (if (Utilities|IsValid (Variables|System|GetmyWidget))
    (Default|Update (Variables|System|GetmyWidget))
    (bind _output_get (Variables|Default|SetshowWidgetCounter (+ (Variables|Default|GetshowWidgetCounter) (Utilities|Time|GetWorldDeltaSeconds))))
    (if (> _output_get 1e+01)
      (Widget|RemovefromParent (Variables|System|GetmyWidget))
      (Variables|System|SetmyWidget 0))))

(event Game|Damage|EventAnyDamage
  (params (Damage :type Float%20%28single-precision%29) (DamageType :type Damage%20Type%20Object%20Reference) (InstigatedBy :type Controller%20Object%20Reference) (DamageCauser :type Actor%20Object%20Reference))
  (CallFunction|ShowWidget)
  (Variables|Default|SetshowWidgetCounter 0.0)
  (bind _output_get (Variables|System|Sethp (- (Variables|System|Gethp) (Math|Float|Truncate Damage))))
  (Default|SetHPBer (Variables|System|GetmyWidget) _output_get (Variables|Default|GetmaxHP))
  (Effects|SpawnEmitteratLocation "/Game/VFXExplosions/Particles/P_Explo_Grenade.P_Explo_Grenade" (Transformation|GetActorLocation))
  (if (<= (Variables|System|Gethp) 0)
    (CallFunction|DieOverride)
    (Default|GetEXP (Variables|Default|Getmarisa) (Variables|Default|Getexp))
    (Widget|RemovefromParent (Variables|System|GetmyWidget))
    (Variables|System|SetmyWidget 0)))

(fn ConstructionScript)

(fn DieOverride)

(fn AttackOverride
  (params (actor :type Actor%20Object%20Reference)))

(fn DestroyEnemy
  (Actor|DestroyActor))

(fn ShowWidget
  (if (or (not (Utilities|IsValid (Variables|System|GetmyWidget))) (== (Variables|System|GetmyWidget) 0))
    (bind _returnvalue (UserInterface|CreateWidget "/Game/BluePrints/UMG/EnemyStatosWidget_BP.EnemyStatosWidget_BP_C"))
    (UserInterface|Viewport|AddtoViewport _returnvalue 0)
    (bind _output_get (Variables|System|SetmyWidget _returnvalue))
    (Default|Initialize _output_get self (Variables|Default|GetyOffset) (Variables|Default|Getname))))

(fn Attack
  (params (actor :type Actor%20Object%20Reference))
  (CallFunction|AttackOverride actor)
  (return 0))