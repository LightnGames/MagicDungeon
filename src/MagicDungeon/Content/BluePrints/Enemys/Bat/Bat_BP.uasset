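; Bat enemy that attacks Marisa when she enters its Box trigger and flags its animation Blueprint on death.
; An Attack timeline turns the mesh toward her, then AttackAction triggers the attack animation and spawns EnemyAttack_BP ahead with base attack damage.
; After a short delay, a second timeline eases the mesh back to rest before clearing the Attacking guard.
; Yaw offsets of 90 degrees compensate for the mesh's orientation.
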(event OnComponentBeginOverlap(Box)
  (params (OtherActor :type Actor%20Object%20Reference) (OtherComp :type Primitive%20Component%20Object%20Reference) (OtherBodyIndex :type Integer) (bFromSweep :type Boolean) (SweepResult :type Hit%20Result%20Structure%20%28by%20ref%29))
  (bind _asmarisa_bp (Utilities|Casting|CastToMarisa_BP OtherActor))
  (if (not (Variables|Default|Getattacking))
    (Variables|Default|Setattacking true)
    (Timeline|attack PlayFromStart
      (:Update
        (Transformation|SetWorldRotation (Variables|Character|GetMesh) (Math|Interpolation|RInterpTo (Transformation|GetWorldRotation (Variables|Character|GetMesh)) (Math|Rotator|MakeRotator 0.0 0.0 (+ (.yaw (Math|Rotator|FindLookatRotation (Transformation|GetWorldLocation (Variables|Character|GetMesh)) (Transformation|GetActorLocation _asmarisa_bp))) -9e+01)) (Utilities|Time|GetWorldDeltaSeconds) 8.0) false false))
      (:Finished
        (|attackAction _asmarisa_bp)
        (Utilities|FlowControl|Delay 0.5)
        (Timeline|タイムライン_0 PlayFromStart
          (:Update
            (Transformation|SetRelativeRotation (Variables|Character|GetMesh) (Math|Interpolation|RInterpTo (Variables|/Script/Engine.SceneComponent|GetRelativeRotation (Variables|Character|GetMesh)) "0,-90.000000, 0" (Utilities|Time|GetWorldDeltaSeconds) 8.0) false false))
          (:Finished
            (Variables|Default|Setattacking false)))))))

(event EventBeginPlay
  (|CallParentFunction)
  (bind _output_get (Variables|Default|SetmyABP (.AsBat%20ABP (Utilities|Casting|CastToBat_ABP (Components|SkeletalMesh|GetAnimInstance (Variables|Character|GetMesh))))))
  (Variables|/Game/BluePrints/Enemys/Bat/Bat_ABP.Bat_ABP_C|Setenemy _output_get self))

(event EventActorBeginOverlap
  (params (OtherActor :type Actor%20Object%20Reference)))

(event EventTick
  (params (DeltaSeconds :type Float%20%28single-precision%29))
  (|CallParentFunction DeltaSeconds))

(event EventDieOverride
  (Variables|/Game/BluePrints/Enemys/Bat/Bat_ABP.Bat_ABP_C|Setdie (Variables|Default|GetmyABP) true))

(fn ConstructionScript
  (|CallParentFunction))