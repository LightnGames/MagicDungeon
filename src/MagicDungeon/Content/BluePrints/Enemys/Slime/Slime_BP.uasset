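; Slime enemy Blueprint that specializes a parent enemy class with its own attack and death behavior.
; On BeginPlay it caches its Slime_ABP anim instance and passes itself to it as Enemy.
; The attack override stores the target, flags the attack animation and immediately spawns a non-player-side EnemyAttack_BP just ahead using base attack points.
; The death override only sets the animation's Die flag.
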(event EventBeginPlay
  (|CallParentFunction)
  (bind _asslime_abp (Utilities|Casting|CastToSlime_ABP (Components|SkeletalMesh|GetAnimInstance (Variables|Character|GetMesh))))
  (bind _output_get (Variables|Default|SetmyABP _asslime_abp))
  (Variables|/Game/BluePrints/Enemys/Slime/Slime_ABP.Slime_ABP_C|Setenemy _output_get self))

(event EventTick
  (params (DeltaSeconds :type Float%20%28single-precision%29))
  (|CallParentFunction DeltaSeconds))

(event EventDieOverride
  (Variables|/Game/BluePrints/Enemys/Slime/Slime_ABP.Slime_ABP_C|Setdie (Variables|Default|GetmyABP) true))

(event EventAttackOverride
  (params (actor :type Actor%20Object%20Reference))
  (bind _returnvalue (Transformation|GetActorRotation))
  (Variables|Default|SetnowTarget actor)
  (Variables|/Game/BluePrints/Enemys/Slime/Slime_ABP.Slime_ABP_C|Setattack (Variables|Default|GetmyABP) true)
  (Game|SpawnActorfromClass "/Game/BluePrints/Magics/EnemyAttack_BP.EnemyAttack_BP_C" (Math|Transform|MakeTransform (+ (Transformation|GetActorLocation) (* (Math|Vector|GetForwardVector _returnvalue) 1e+02)) _returnvalue "1,1,1") "Undefined" 0 0.0 0.0 (Variables|Default|GetbaseAttackPoint) 0 false))

(fn ConstructionScript
  (|CallParentFunction))