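; Box enemy that fires attacks while Marisa_BP is inside either of its two trigger boxes.
; Each box's overlap plays its own timeline, whose event calls Attack, and end overlap stops that timeline.
; Attack spawns an enemy-side EnemyAttack_BP ahead of the actor along that box's forward vector, with damage from BaseAttackPoint.
; DieOverride calls DestroyEnemy.
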(event OnComponentEndOverlap(Box)
  (params (OtherActor :type Actor%20Object%20Reference) (OtherComp :type Primitive%20Component%20Object%20Reference) (OtherBodyIndex :type Integer))
  (Utilities|Casting|CastToMarisa_BP OtherActor)
  (Timeline|タイムライン_1 Stop
    (:event
      (Utilities|Attack (Variables|Default|Gettarget) (Variables|Default|GetBox)))))

(event OnComponentEndOverlap(Box1)
  (params (OtherActor :type Actor%20Object%20Reference) (OtherComp :type Primitive%20Component%20Object%20Reference) (OtherBodyIndex :type Integer))
  (Utilities|Casting|CastToMarisa_BP OtherActor)
  (Timeline|タイムライン_0 Stop
    (:event
      (Utilities|Attack (Variables|Default|Gettarget) (Variables|Default|GetBox1)))))

(event OnComponentBeginOverlap(Box)
  (params (OtherActor :type Actor%20Object%20Reference) (OtherComp :type Primitive%20Component%20Object%20Reference) (OtherBodyIndex :type Integer) (bFromSweep :type Boolean) (SweepResult :type Hit%20Result%20Structure%20%28by%20ref%29))
  (bind _asmarisa_bp (Utilities|Casting|CastToMarisa_BP OtherActor))
  (Variables|Default|Settarget _asmarisa_bp)
  (Timeline|タイムライン_1 Play
    (:event
      (Utilities|Attack (Variables|Default|Gettarget) (Variables|Default|GetBox)))))

(event OnComponentBeginOverlap(Box1)
  (params (OtherActor :type Actor%20Object%20Reference) (OtherComp :type Primitive%20Component%20Object%20Reference) (OtherBodyIndex :type Integer) (bFromSweep :type Boolean) (SweepResult :type Hit%20Result%20Structure%20%28by%20ref%29))
  (bind _asmarisa_bp (Utilities|Casting|CastToMarisa_BP OtherActor))
  (Variables|Default|Settarget _asmarisa_bp)
  (Timeline|タイムライン_0 Play
    (:event
      (Utilities|Attack (Variables|Default|Gettarget) (Variables|Default|GetBox1)))))

(event EventDieOverride
  (CallFunction|DestroyEnemy))

(event EventBeginPlay
  (|CallParentFunction))

(event EventTick
  (params (DeltaSeconds :type Float%20%28single-precision%29))
  (|CallParentFunction DeltaSeconds))

(fn ConstructionScript
  (|CallParentFunction))