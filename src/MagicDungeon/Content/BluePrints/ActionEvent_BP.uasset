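; ActionEvent_BP is an event actor that shows an on-screen icon while Marisa_BP is inside its Box trigger.
; Box begin overlap creates an EventIconWidget_BP with the actor, WidgetPoint's relative location and Widget2dTexture, unless HideEventIcon is set.
; Tick calls Update on the active widget, and end overlap removes it and clears the reference.
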(event OnComponentEndOverlap(Box)
  (params (OtherActor :type Actor%20Object%20Reference) (OtherComp :type Primitive%20Component%20Object%20Reference) (OtherBodyIndex :type Integer))
  (Utilities|Casting|CastToMarisa_BP OtherActor)
  (CallFunction|RemoveWidget))

(event OnComponentBeginOverlap(Box)
  (params (OtherActor :type Actor%20Object%20Reference) (OtherComp :type Primitive%20Component%20Object%20Reference) (OtherBodyIndex :type Integer) (bFromSweep :type Boolean) (SweepResult :type Hit%20Result%20Structure%20%28by%20ref%29))
  (Utilities|Casting|CastToMarisa_BP OtherActor)
  (CallFunction|ShowWidget))

(event EventBeginPlay)

(event EventActorBeginOverlap
  (params (OtherActor :type Actor%20Object%20Reference)))

(event EventTick
  (params (DeltaSeconds :type Float%20%28single-precision%29))
  (bind _iconwidget (Variables|Default|GeticonWidget))
  (if (!= _iconwidget 0)
    (Default|Update _iconwidget)))

(fn ConstructionScript)

(fn ShowWidget
  (if (not (Variables|Default|GethideEventIcon))
    (bind _returnvalue (UserInterface|CreateWidget "/Game/BluePrints/UMG/EventIconWidget_BP.EventIconWidget_BP_C" 0 self (Variables|/Script/Engine.SceneComponent|GetRelativeLocation (Variables|Default|GetWidgetPoint)) (Variables|Default|Getwidget2dTexture)))
    (UserInterface|Viewport|AddtoViewport _returnvalue 0)
    (Variables|Default|SeticonWidget _returnvalue)))

(fn RemoveWidget
  (if (!= (Variables|Default|GeticonWidget) 0)
    (Widget|RemovefromParent (Variables|Default|GeticonWidget))
    (Variables|Default|SeticonWidget 0)))