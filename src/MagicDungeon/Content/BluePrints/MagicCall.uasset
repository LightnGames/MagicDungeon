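; MagicCall is the casting actor for Marisa's standby magic, registering itself with her anim Blueprint and zeroing her crouched walk speed on BeginPlay.
; CallFinish triggers FinishCall, which spawns the spell's emitter at MagicStenby's targeting decal, passes its MP value to MPUpDown, removes the decal and restores speed.
; After a short delay, it clears MagicStenby's current call and spawns a fresh decal.
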(event EventFinishCall
  (bind _magicstenby (Variables|Default|GetmagicStenby))
  (bind _magicstenby_2 (Variables|Default|GetmagicStenby))
  (bind _marisa (Variables|Default|Getmarisa))
  (bind _nowdecal (Variables|/Game/BluePrints/MagicStenby.MagicStenby_C|GetnowDecal _magicstenby_2))
  (bind _stenbymagic (Variables|/Game/BluePrints/Marisa/Marisa_BP.Marisa_BP_C|GetstenbyMagic _marisa))
  (bind (_name _mp _damage _maxdistance _areascale _level _exp _image _emitter) (Utilities|Struct|BreakMagicDatas _stenbymagic))
  (Game|SpawnActorfromClass _emitter (Math|Transform|MakeTransform (Transformation|GetActorLocation _nowdecal) (Transformation|GetActorRotation _nowdecal) "1,1,1") "Undefined" 0 _marisa true _stenbymagic)
  (Default|MPUpDown (Variables|Default|Getmarisa) _mp)
  (Default|DeleteNowDecal (Variables|Default|GetmagicStenby))
  (Variables|/Script/Engine.CharacterMovementComponent|SetMaxWalkSpeedCrouched (Variables|/Script/Engine.Character|GetCharacterMovement (Variables|Default|Getmarisa)) (Variables|Default|GetsaveWalkSpeed))
  (Utilities|FlowControl|Delay 0.5)
  (if (Utilities|IsValid _magicstenby)
    (Variables|/Game/BluePrints/MagicStenby.MagicStenby_C|SetnowMagicCall _magicstenby 0)
    (Default|SpawnNowDecal _magicstenby)))

(event EventBeginPlay
  (bind _marisa (Variables|Default|Getmarisa))
  (bind _charactermovement (Variables|/Script/Engine.Character|GetCharacterMovement _marisa))
  (Variables|/Game/BluePrints/Marisa/Marisa_ABP.Marisa_ABP_C|SetmagicCall (Variables|/Game/BluePrints/Marisa/Marisa_BP.Marisa_BP_C|GetmarisaABP _marisa) self)
  (Variables|Default|SetsaveWalkSpeed (Variables|/Script/Engine.CharacterMovementComponent|GetMaxWalkSpeedCrouched _charactermovement))
  (Variables|/Script/Engine.CharacterMovementComponent|SetMaxWalkSpeedCrouched _charactermovement 0.0))

(event EventActorBeginOverlap
  (params (OtherActor :type Actor%20Object%20Reference)))

(event EventTick
  (params (DeltaSeconds :type Float%20%28single-precision%29)))

(fn ConstructionScript)

(fn CallFinish
  (CallFunction|FinishCall))