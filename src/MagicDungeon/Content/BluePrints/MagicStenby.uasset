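; An actor that puts Marisa into a magic standby stance, from which the readied spell can be cast.
; BeginPlay crouches her, enables the battle-standing animation flag and spawns an aiming decal, while Tick smoothly turns her to the camera rig's yaw.
; MagicCall spawns a single MagicCall actor if MP covers the spell's cost.
; Finish, allowed only when no call is active, undoes the stance and destroys the decal and actor.
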(event EventBeginPlay
  (bind _marisa (Variables|Default|Getmarisa))
  (Variables|/Script/Engine.CharacterMovementComponent|SetbOrientRotationToMovement (Variables|/Script/Engine.Character|GetCharacterMovement _marisa) false)
  (Character|Crouch _marisa)
  (Variables|/Game/BluePrints/Marisa/Marisa_ABP.Marisa_ABP_C|SetbuttleStanding (Variables|/Game/BluePrints/Marisa/Marisa_BP.Marisa_BP_C|GetmarisaABP _marisa) true)
  (CallFunction|SpawnNowDecal))

(event EventActorBeginOverlap
  (params (OtherActor :type Actor%20Object%20Reference)))

(event EventTick
  (params (DeltaSeconds :type Float%20%28single-precision%29))
  (bind _marisa (Variables|Default|Getmarisa))
  (Transformation|SetActorRotation _marisa (Math|Interpolation|RInterpTo (Transformation|GetActorRotation _marisa) (Math|Rotator|MakeRotator 0.0 0.0 (.yaw (Transformation|GetWorldRotation (Variables|/Game/BluePrints/Marisa/Marisa_BP.Marisa_BP_C|GetCameraRig _marisa)))) (Utilities|Time|GetWorldDeltaSeconds) 4.0)))

(fn ConstructionScript)

(fn Finish
  (bind _marisa (Variables|Default|Getmarisa))
  (if (== (Variables|Default|GetnowMagicCall) 0)
    (Variables|/Script/Engine.CharacterMovementComponent|SetbOrientRotationToMovement (Variables|/Script/Engine.Character|GetCharacterMovement _marisa) true)
    (Character|UnCrouch _marisa)
    (Variables|/Game/BluePrints/Marisa/Marisa_ABP.Marisa_ABP_C|SetbuttleStanding (Variables|/Game/BluePrints/Marisa/Marisa_BP.Marisa_BP_C|GetmarisaABP _marisa) false)
    (CallFunction|DeleteNowDecal)
    (Variables|/Game/BluePrints/Marisa/Marisa_BP.Marisa_BP_C|SetmagicStenby (Variables|Default|Getmarisa) 0)
    (Actor|DestroyActor)))

(fn MagicCall
  (bind _marisa (Variables|Default|Getmarisa))
  (if (and (== (Variables|Default|GetnowMagicCall) 0) (>= (.mp (Variables|/Game/BluePrints/Marisa/Marisa_BP.Marisa_BP_C|GetplayerData _marisa)) (.mp (Variables|/Game/BluePrints/Marisa/Marisa_BP.Marisa_BP_C|GetstenbyMagic _marisa))))
    (bind _returnvalue (Game|SpawnActorfromClass "/Game/BluePrints/MagicCall.MagicCall_C" (Math|Transform|MakeTransform "0, 0, 0" "0, 0, 0" "1,1,1") "Undefined" 0 (Variables|Default|Getmarisa) self))
    (Variables|Default|SetnowMagicCall _returnvalue)))

(fn DeleteNowDecal
  (if (Utilities|IsValid (Variables|Default|GetnowDecal))
    (Actor|DestroyActor (Variables|Default|GetnowDecal))))

(fn SpawnNowDecal
  (bind _returnvalue (Game|SpawnActorfromClass "/Game/BluePrints/MagicDecal.MagicDecal_C" (Math|Transform|MakeTransform "0, 0, 0" "0, 0, 0" "1,1,1") "Undefined" 0 (Variables|Default|Getmarisa) 0))
  (Variables|Default|SetnowDecal _returnvalue))