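; FlooingSwitch_BP is a one-shot floor switch gimmick that signals a linked door actor when something overlaps its Box.
; The overlap plays the switch animation and a FadeColor timeline that shifts the decal's dynamic material Color from orange-red to blue.
; When the fade finishes, it sends a "Door" GimicEventMessage to DoorActor and sets Off, which blocks further triggers.
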(event OnComponentBeginOverlap(Box)
  (params (OtherActor :type Actor%20Object%20Reference) (OtherComp :type Primitive%20Component%20Object%20Reference) (OtherBodyIndex :type Integer) (bFromSweep :type Boolean) (SweepResult :type Hit%20Result%20Structure%20%28by%20ref%29))
  (if (not (Variables|Default|Getoff))
    (Components|Animation|PlayAnimation (Variables|SkeletalMeshActor|GetSkeletalMeshComponent) "/Game/3D/Gimic/FlooringSwitch/FlooingSwitch_Anim.FlooingSwitch_Anim" false)
    (bind _value (Timeline|FadeColor Play)
      (:Update
        (Rendering|Material|SetVectorParameterValue (.AsMaterial%20Instance%20Dynamic (Utilities|Casting|CastToMaterialInstanceDynamic (Variables|/Script/Engine.DecalComponent|GetDecalMaterial (Variables|Default|GetDecal)))) "Color" (Utilities|Struct|MakeLinearColor (.X (Math|Vector|BreakVector (Math|Interpolation|Ease "Linear" _value "1.000000,0.200000,0" "0,0.200000,1.000000"))) (.Y (Math|Vector|BreakVector (Math|Interpolation|Ease "Linear" _value "1.000000,0.200000,0" "0,0.200000,1.000000"))) (.Z (Math|Vector|BreakVector (Math|Interpolation|Ease "Linear" _value "1.000000,0.200000,0" "0,0.200000,1.000000"))) 0.0) :!class /Script/Engine.MaterialInstanceDynamic))
      (:Finished
        (Class|StageGimicInterface|GimicEvent(Message) (Variables|Default|GetdoorActor) "Door" 0.0)
        (Variables|Default|Setoff true)))))

(event EventBeginPlay
  (Rendering|Material|CreateDynamicMaterialInstance (Variables|Default|GetDecal) :!class /Script/Engine.DecalComponent))

(event EventActorBeginOverlap
  (params (OtherActor :type Actor%20Object%20Reference)))

(event EventTick
  (params (DeltaSeconds :type Float%20%28single-precision%29)))

(fn ConstructionScript)