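; King_obelisk_BP is an obelisk gimmick that lights up with fire when it takes any damage, then resets.
; BeginPlay creates a dynamic material on the mesh and zeroes its Alpha and the Fire scale.
; Damage plays the Fade timeline, driving both values together, then a TimeUp timeline acts as a delay before Initialize resets them.
; Tick keeps Fire's world rotation at zero so it stays upright.
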(event EventTick
  (params (DeltaSeconds :type Float%20%28single-precision%29))
  (Transformation|SetWorldRotation (Variables|Default|GetFire) "0, 0, 0" false false))

(event EventBeginPlay
  (bind _returnvalue (Rendering|Material|CreateDynamicMaterialInstance (Variables|Default|GetStaticMesh) 2 "/Game/TopDownDungeons/Deco/Materials/deco1_Mat_Inst.deco1_Mat_Inst" :!class /Script/Engine.PrimitiveComponent))
  (Variables|Default|SetmaterialInstance _returnvalue)
  (Utilities|Initialize))

(event Game|Damage|EventAnyDamage
  (params (Damage :type Float%20%28single-precision%29) (DamageType :type Damage%20Type%20Object%20Reference) (InstigatedBy :type Controller%20Object%20Reference) (DamageCauser :type Actor%20Object%20Reference))
  (bind _alpha (Timeline|fade PlayFromStart)
    (:Update
      (Rendering|Material|SetScalarParameterValue (Variables|Default|GetmaterialInstance) "Alpha" _alpha :!class /Script/Engine.MaterialInstanceDynamic)
      (Transformation|SetRelativeScale3D (Variables|Default|GetFire) (Math|Vector|MakeVector _alpha _alpha _alpha)))
    (:Finished
      (Timeline|TimeUp PlayFromStart
        (:Finished
          (Utilities|Initialize))))))

(fn ConstructionScript)