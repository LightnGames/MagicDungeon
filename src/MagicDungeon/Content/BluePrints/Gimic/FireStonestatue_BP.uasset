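; FireStonestatue_BP is a gimmick stone statue that lights up when it receives a Fire event and signals a door.
; Its orb glow lights are hidden at BeginPlay.
; On a "Fire" GimicEvent, OnSwitch shows the lights and swaps the statue's second material to M_DemonStatue_Fire, then a "Door" event is sent to GimicParent.
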(event EventBeginPlay
  (Rendering|SetVisibility (Variables|Default|GetP_OrbGlowLights) false false))

(event EventTick
  (params (DeltaSeconds :type Float%20%28single-precision%29)))

(event EventGimicEvent
  (params (string :type String) (value :type Float%20%28single-precision%29))
  (if (Utilities|Enum|Equal(Enum) string "Fire")
    (CallFunction|OnSwitch)
    (Default|GimicEvent (Variables|Default|GetgimicParent) "Door" 0.0)))

(fn ConstructionScript)

(fn OnSwitch
  (Rendering|SetVisibility (Variables|Default|GetP_OrbGlowLights) true false)
  (Rendering|Material|SetMaterial (Variables|Debug|GetStaticMeshComponent) 1 "/Game/Environment/Materials/Misc/M_DemonStatue_Fire.M_DemonStatue_Fire"))