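; B2Door is a gimmick door that slides open after receiving enough trigger events.
; Each GimicEvent carrying the "Door" string increments Counter, and reaching SetCounter plays the Open timeline.
; Every timeline update moves the actor a fixed step along its right vector without sweep, so travel distance depends on the update count.
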(event EventBeginPlay)

(event EventActorBeginOverlap
  (params (OtherActor :type Actor%20Object%20Reference)))

(event EventTick
  (params (DeltaSeconds :type Float%20%28single-precision%29)))

(event EventGimicEvent
  (params (string :type String) (value :type Float%20%28single-precision%29))
  (if (Utilities|Enum|Equal(Enum) string "Door")
    (bind _result (Math|Integer|IncrementInt (Variables|Default|Getcounter))
      (:%20%20
        (if (>= _result (Variables|Default|GetsetCounter))
          (Timeline|Open Play
            (:Update
              (Transformation|AddActorWorldOffset (* (Math|Vector|GetRightVector (Transformation|GetActorRotation)) 2.0)))))))))

(fn ConstructionScript)