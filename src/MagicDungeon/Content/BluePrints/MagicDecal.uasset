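; MagicDecal is an aiming decal that marks where Marisa's camera points and shows the area size of her standby magic.
; Each tick a long visibility trace from the camera moves the actor to the hit location, showing the decal only on a blocking hit.
; The decal starts at zero scale and eases uniformly toward StenbyMagic's areaScale by a tenth of the remaining difference per tick, so the easing is frame-rate dependent.
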(event EventBeginPlay
  (Transformation|SetRelativeScale3D (Variables|Default|GetDecal) (Math|Vector|MakeVector 0.0 0.0 0.0)))

(event EventTick
  (params (DeltaSeconds :type Float%20%28single-precision%29))
  (bind _decal (Variables|Default|GetDecal))
  (bind _marisa (Variables|Default|Getmarisa))
  (bind _camera (Variables|/Game/BluePrints/Marisa_BP.Marisa_BP_C|GetCamera _marisa))
  (bind _returnvalue (Transformation|GetWorldLocation _camera))
  (|デカールサイズをセット _marisa)
  (bind _outhit (Collision|LineTraceByChannel _returnvalue (+ _returnvalue (* (Math|Vector|GetForwardVector (Transformation|GetWorldRotation _camera)) 100000)) "TraceTypeQuery1" false 0 "None"))
  (Transformation|SetActorLocation (.Location (Collision|BreakHitResult _outhit)) false false)
  (if (.bBlockingHit (Collision|BreakHitResult _outhit))
    (Rendering|SetVisibility _decal true false)
    (else
      (Rendering|SetVisibility _decal false false))))

(fn ConstructionScript)