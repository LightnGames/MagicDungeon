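; PlayerAttack is an actor Blueprint representing an attack by the player character Marisa, holding her in place until the attack finishes.
; On BeginPlay it registers itself as Attacking on her animation Blueprint, saves her max walk speed and sets it to zero.
; AttackFinish restores the saved speed, then calls FinishCall, which waits briefly, clears Marisa's Attack reference and destroys the actor.
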(event EventBeginPlay
  (bind _marisa (Variables|Default|Getmarisa))
  (bind _charactermovement (Variables|/Script/Engine.Character|GetCharacterMovement _marisa))
  (Variables|/Game/BluePrints/Marisa/Marisa_ABP.Marisa_ABP_C|Setattacking (Variables|/Game/BluePrints/Marisa/Marisa_BP.Marisa_BP_C|GetmarisaABP _marisa) self)
  (Variables|Default|SetsaveWalkSpeed (Variables|/Script/Engine.CharacterMovementComponent|GetMaxWalkSpeed _charactermovement))
  (Variables|/Script/Engine.CharacterMovementComponent|SetMaxWalkSpeed _charactermovement 0.0))

(event EventActorBeginOverlap
  (params (OtherActor :type Actor%20Object%20Reference)))

(event EventTick
  (params (DeltaSeconds :type Float%20%28single-precision%29)))

(event EventFinishCall
  (Utilities|FlowControl|Delay 0.35)
  (Variables|/Game/BluePrints/Marisa/Marisa_BP.Marisa_BP_C|Setattack (Variables|Default|Getmarisa) 0)
  (Actor|DestroyActor))

(fn ConstructionScript)

(fn AttackFinish
  (Variables|/Script/Engine.CharacterMovementComponent|SetMaxWalkSpeed (Variables|/Script/Engine.Character|GetCharacterMovement (Variables|Default|Getmarisa)) (Variables|Default|GetsaveWalkSpeed))
  (CallFunction|FinishCall))