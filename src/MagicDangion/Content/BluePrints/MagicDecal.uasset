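; MagicDecal is an actor with a decal that marks where the Marisa reference's camera is aiming on world-static geometry.
; Each tick it traces forward from that camera, moves to the hit location, and shows the decal only on a blocking hit.
; On BeginPlay, it zeroes the decal's scale, then a timeline eases it out toward its saved default scale.
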(event EventBeginPlay
  (Variables|Default|SetdefaultScale (Variables|/Script/Engine.SceneComponent|GetRelativeScale3D (Variables|Default|GetDecal)))
  (Transformation|SetRelativeScale3D (Variables|Default|GetDecal) "0, 0, 0")
  (bind _value (Timeline|ScaleUp Play)
    (:Update
      (Transformation|SetRelativeScale3D (Variables|Default|GetDecal) (Math|Interpolation|Ease "EaseOut" _value (Math|Vector|MakeVector (.X (Math|Vector|BreakVector (Variables|Default|GetdefaultScale))) 0.0 0.0) (Variables|Default|GetdefaultScale) 3.0)))))

(event EventTick
  (params (DeltaSeconds :type Float%20%28single-precision%29))
  (bind _decal (Variables|Default|GetDecal))
  (bind _marisa (Variables|Default|Getmarisa))
  (bind _camera (Variables|/Game/BluePrints/Marisa_BP.Marisa_BP_C|GetCamera _marisa))
  (bind _returnvalue (Transformation|GetWorldLocation _camera))
  (bind _outhit (Collision|LineTraceForObjects _returnvalue (+ _returnvalue (* (Math|Vector|GetForwardVector (Transformation|GetWorldRotation _camera)) 100000)) (Utilities|Array|MakeArray "ObjectTypeQuery1") false 0 "None"))
  (Transformation|SetActorLocation (.Location (Collision|BreakHitResult _outhit)) false false)
  (if (.bBlockingHit (Collision|BreakHitResult _outhit))
    (Rendering|SetVisibility _decal true false)
    (else
      (Rendering|SetVisibility _decal false false))))

(fn ConstructionScript)