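; MagicCall handles one cast of Marisa's standby spell (StenbyMagic).
; On BeginPlay it registers with her anim Blueprint and zeroes her crouched walk speed for the cast.
; CallFinish triggers FinishCall, which spawns the spell's emitter at the targeting decal, deducts MP, removes the decal and restores speed.
; After a short delay, it clears itself from MagicStenby and respawns the decal.
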(event EventFinishCall
  (bind _magicstenby (Variables|Default|GetmagicStenby))
  (bind _marisa (Variables|Default|Getmarisa))
  (bind _marisa_2 (Variables|Default|Getmarisa))
  (bind _stenbymagic (Variables|/Game/BluePrints/Marisa_BP.Marisa_BP_C|GetstenbyMagic _marisa))
  (bind (_name _mp _damage _level _exp _image _emitter) (Utilities|Struct|BreakMagicDatas _stenbymagic))
  (Game|SpawnActorfromClass _emitter (Math|Transform|MakeTransform (Transformation|GetActorLocation (Variables|/Game/BluePrints/MagicStenby.MagicStenby_C|GetnowDecal (Variables|Default|GetmagicStenby))) "0, 0, 0" "1,1,1") "Undefined" 0 _marisa true _stenbymagic)
  (Variables|/Game/BluePrints/Marisa_BP.Marisa_BP_C|Setmp _marisa_2 (- (Variables|/Game/BluePrints/Marisa_BP.Marisa_BP_C|Getmp _marisa_2) _mp))
  (Default|DeleteNowDecal (Variables|Default|GetmagicStenby))
  (Variables|/Script/Engine.CharacterMovementComponent|SetMaxWalkSpeedCrouched (Variables|/Script/Engine.Character|GetCharacterMovement (Variables|Default|Getmarisa)) (Variables|Default|GetsaveWalkSpeed))
  (Utilities|FlowControl|Delay 0.5)
  (if (Utilities|IsValid _magicstenby)
    (Variables|/Game/BluePrints/MagicStenby.MagicStenby_C|SetnowMagicCall _magicstenby 0)
    (Default|SpawnNowDecal _magicstenby)))

(event EventBeginPlay
  (bind _marisa (Variables|Default|Getmarisa))
  (bind _charactermovement (Variables|/Script/Engine.Character|GetCharacterMovement _marisa))
  (Variables|/Game/BluePrints/Marisa_ABP.Marisa_ABP_C|SetmagicCall (Variables|/Game/BluePrints/Marisa_BP.Marisa_BP_C|GetmarisaABP _marisa) self)
  (Variables|Default|SetsaveWalkSpeed (Variables|/Script/Engine.CharacterMovementComponent|GetMaxWalkSpeedCrouched _charactermovement))
  (Variables|/Script/Engine.CharacterMovementComponent|SetMaxWalkSpeedCrouched _charactermovement 0.0))

(event EventActorBeginOverlap
  (params (OtherActor :type Actor%20Object%20Reference)))

(event EventTick
  (params (DeltaSeconds :type Float%20%28single-precision%29)))

(fn ConstructionScript)

(fn CallFinish
  (CallFunction|FinishCall))