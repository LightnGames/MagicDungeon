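; Magic actor, likely a base for spells, that deals damage and destroys itself once its particle is no longer valid.
; Hit uses PlayerSIde to target Enemy or Marisa_BP, spawns a damage number widget, then applies MyData damage with ±10% variance.
; The random roll is evaluated separately for widget, damage and debug print, so values can differ.
; SwitchCollision toggles collision by moving the component far below its origin; MagicFinish calls FinishCall.
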(event EventBeginPlay)

(event EventActorBeginOverlap
  (params (OtherActor :type Actor%20Object%20Reference)))

(event EventTick
  (params (DeltaSeconds :type Float%20%28single-precision%29))
  (if (not (and (Utilities|IsValid (Variables|Default|GetmyParticle)) (!= (Variables|Default|GetmyParticle) 0)))
    (Variables|Default|SetmyParticle 0)
    (Actor|DestroyActor)))

(fn ConstructionScript)

(fn MagicFinish
  (CallFunction|FinishCall))

(fn Hit
  (params (target :type Actor%20Object%20Reference))
  (bind _returnvalue (Math|Random|RandomFloatinRange -1.0 1.0))
  (bind _mydata (Variables|Default|GetmyData))
  (bind _returnvalue_2 (Math|Conversions|ToFloat(Integer) (.damage _mydata)))
  (bind _returnvalue_3 (* _returnvalue_2 0.1 _returnvalue))
  (bind _returnvalue_4 (Math|Float|Truncate _returnvalue_3))
  (bind _returnvalue_5 (+ (.damage _mydata) _returnvalue_4))
  (if (Variables|Default|GetplayerSIde)
    (bind _asenemy (Utilities|Casting|CastToEnemy target))
    (|ダメージWidget表示 _asenemy _returnvalue_5
      (:out
        _))
    (else
      (bind _asmarisa_bp (Utilities|Casting|CastToMarisa_BP target))
      (|ダメージWidget表示_2 _asmarisa_bp _returnvalue_5
        (:out
          _))))
  (Game|Damage|ApplyDamage target (Math|Conversions|ToFloat(Integer) _returnvalue_5) 0 0)
  (Development|PrintString (Utilities|String|ToString(Integer) _returnvalue_5)))

(fn SwitchCollision
  (params (set :type Boolean) (target :type Scene%20Component%20Object%20Reference))
  (if set
    (Transformation|SetRelativeLocation target "0, 0,0.000000" false false)
    (else
      (Transformation|SetRelativeLocation target "0, 0,-1000.000000" false false))))